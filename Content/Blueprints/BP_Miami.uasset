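; BP_Miami is an endless-runner road tile that randomizes its road meshes, car lanes and car materials on BeginPlay.
; Two timelines drive the same-direction and oncoming cars by offsetting their world X while the player is alive.
; The Box trigger asks ThirdPersonGameMode to spawn the next tile, then destroys this one after a short delay.
; CarKillZone overlap spawns effects, fractures a destructible car, kills the player, disables input and stops both timelines.
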(event `DeadPlayer`
  (bind _caruup (`self.CarUup`))
  (bind _cardoown (`self.CarDoown`))
  (bind (_returnvalue_x _returnvalue_y _returnvalue_z) (`KismetMathLibrary.BreakVector` (`SceneComponent.K2_GetComponentLocation` _cardoown)))
  (bind (_returnvalue_x_2 _returnvalue_y_2 _returnvalue_z_2) (`KismetMathLibrary.BreakVector` (`SceneComponent.K2_GetComponentLocation` _caruup)))
  ;[1 1 1] Dead Event
  (`|ExecutionSequence`
    (:`then_0`
      ;[1 1 1] Поведение машины
      (bind (_direction _drivey) (`Timeline|Timeline_0` :!via `Stop` :!label _label)
        (:`Update`
          (`SceneComponent.K2_SetWorldLocation` _caruup (`KismetMathLibrary.MakeVector` (+ _drivey _returnvalue_x_2) _returnvalue_y_2 _returnvalue_z_2) false false))))
    (:`then_1`
      ;[1 1 1] Поведение машины встречка
      (bind (_direction_2 _drivey_2) (`Timeline|Timeline_1` :!via `Stop` :!label _label_2)
        (:`Update`
          (`SceneComponent.K2_SetWorldLocation` _cardoown (`KismetMathLibrary.MakeVector` (+ _drivey_2 _returnvalue_x) _returnvalue_y _returnvalue_z) false false))))))

(event `self.ReceiveBeginPlay`
  (bind _asthird_person_character (cast `/Game/ThirdPersonBP/Blueprints/ThirdPersonCharacter` (`GameplayStatics.GetPlayerCharacter` 0)))
  (`|ExecutionSequence`
    (:`then_0`
      (for _array_element (`|MakeArray` (`self.StaticMesh`) (`self.StaticMesh1`) (`self.StaticMesh2`) (`self.StaticMesh3`))
        (`StaticMeshComponent.SetStaticMesh` _array_element (`self.GetRandomRoadMesh`))
        (`SceneComponent.K2_SetWorldLocation` (`self.CarUup`) (`self.GetRandomLineLocation`) false false)
        (`SceneComponent.K2_SetWorldLocation` (`self.CarDoown`) (`self.GetRandomLineLocation_CAR`) false false)
        (`self.RandomMaterialCar` (`self.DestructibleMC1`) (`self.DestructibleMC2`))))
    (:`then_1`
      (bind _is_dead_ (`/Game/ThirdPersonBP/Blueprints/ThirdPersonCharacter.is Dead?` _asthird_person_character))
      (if (not _is_dead_)
        (goto _label_2 :!via `PlayFromStart`)))
    (:`then_2`
      (if (not _is_dead_)
        (goto _label :!via `PlayFromStart`)))))

(event `self.Box.OnComponentBeginOverlap`
  (params (OverlappedComponent :type "PrimitiveComponent Object Reference") (OtherActor :type "Actor Object Reference") (OtherComp :type "PrimitiveComponent Object Reference") (OtherBodyIndex :type Integer) (bFromSweep :type Boolean) (SweepResult :type "HitResult Structure (by ref)"))
  ;[1 1 1] SPAWN NEW TILE ROAD
  (cast `/Game/ThirdPersonBP/Blueprints/ThirdPersonCharacter` OtherActor)
  (bind _asthird_person_game_mode (cast `/Game/ThirdPersonBP/Blueprints/ThirdPersonGameMode` (`GameplayStatics.GetGameMode`)))
  (`/Game/ThirdPersonBP/Blueprints/ThirdPersonGameMode.SpawnTileRoad` _asthird_person_game_mode)
  (`KismetSystemLibrary.Delay` 2.0)
  (`self.K2_DestroyActor`))

(event `self.Car kill zone.OnComponentBeginOverlap`
  (params (OverlappedComponent :type "PrimitiveComponent Object Reference") (OtherActor :type "Actor Object Reference") (OtherComp :type "PrimitiveComponent Object Reference") (OtherBodyIndex :type Integer) (bFromSweep :type Boolean) (SweepResult :type "HitResult Structure (by ref)"))
  (bind _returnvalue (`SceneComponent.K2_GetComponentLocation` (`self.CarUup`)))
  ;[1 1 1] Dead because of cars
  (bind _asthird_person_character (cast `/Game/ThirdPersonBP/Blueprints/ThirdPersonCharacter` OtherActor))
  (for _array_element (`self.ParticleList`)
    (`GameplayStatics.SpawnEmitterAtLocation` _array_element (`KismetMathLibrary.MakeVector` (- (.x _returnvalue) 250.0) (.y _returnvalue) (.z _returnvalue)) (struct) (3.0 3.0 3.0)))
  (`DestructibleComponent.ApplyRadiusDamage` (`self.DestructibleMC1`) 1.0 _returnvalue 10.0 50000.0 true)
  (`/Game/ThirdPersonBP/Blueprints/ThirdPersonCharacter.DeadPlayer` _asthird_person_character)
  (`self.DeadPlayer`)
  (`self.DisableInput` (`GameplayStatics.GetPlayerCharacter` 0) (`GameplayStatics.GetPlayerController` 0))
  (`self.DisableInput` _asthird_person_character (`GameplayStatics.GetPlayerController` 0)))

(fn `UserConstructionScript`)