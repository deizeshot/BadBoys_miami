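; Helicopter actor that shadows the player from above, snapping every tick to a fixed offset from the player character's location.
; On BeginPlay it calls AnimationHelio, which plays a timeline to spin two meshes, likely the main and tail rotors.
; The timeline's Rotater track is applied as a local rotation delta on each update, as yaw for one mesh and pitch for the other.
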(event `self.ReceiveBeginPlay`
  (bind (_direction _rotater) (`Timeline|Helicopter_rotate_light` :!via `PlayFromStart`)
    (:`Update`
      (`SceneComponent.K2_AddLocalRotation` (`self.Helico_game_03v`) (`KismetMathLibrary.MakeRotator` 0.0 0.0 _rotater) false false)
      (`SceneComponent.K2_AddLocalRotation` (`self.Helico_game_03v_Box05`) (`KismetMathLibrary.MakeRotator` 0.0 _rotater) false false))))

(event `self.ReceiveTick`
  (params (DeltaSeconds :type "Float (single-precision)"))
  (`self.K2_SetActorLocation` (+ (`self.K2_GetActorLocation` (`GameplayStatics.GetPlayerCharacter` 0)) (2500.0 -500.0 2000.0))))

(fn `UserConstructionScript`)